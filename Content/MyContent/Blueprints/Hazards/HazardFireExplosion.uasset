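; HazardFireExplosion is a hazard Blueprint that produces a fiery explosion.
; Its DoEffects event spawns the explosion particle emitter just above the mesh and fires a RadialForce impulse.
; It then plays the explosion sound through MyGameState rather than directly on the actor.
; Nothing in this graph calls DoEffects, and the construction script only runs the parent's.
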(event Custom|DoEffects
  ;[1 1 1] Spawn the emitter and impulse damage and play sound
  (Effects|SpawnEmitteratLocation "/Game/MyContent/Particles/P_HazardFireExplosion.P_HazardFireExplosion" (+ (Transformation|GetWorldLocation (Variables|Character|GetMesh)) "0.000000,0.000000,10.000000"))
  (Class|RadialForceComponent|FireImpulse (Variables|Default|GetRadialForce))
  (bind _asmy_game_state (Utilities|Casting|CastToMyGameState (Game|GetGameState)))
  (Default|PlaySound _asmy_game_state "/Game/MyContent/Audio/FX/FX_Explosion.FX_Explosion"))

(event EventBeginPlay
  (|CallParentFunction))

(event EventActorBeginOverlap
  (params (OtherActor :type Actor%20Object%20Reference)))

(event EventTick
  (params (DeltaSeconds :type Float%20%28single-precision%29))
  (|CallParentFunction 0.0))

(fn ConstructionScript
  (|CallParentFunction))