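; Game State Blueprint that runs a floor's combat loop, switching between playing, menu, floor cleared and player dead states.
; On BeginPlay it creates the HUDs, gathers all enemies, activates their AI via Blackboard keys and applies saved audio volumes.
; Enemy deaths shrink the list, announcing the remaining count or notifying the FloorManager once empty.
; It also handles player death, the in-game menu and subtitled audio playback.
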(event Custom|PlaySound
  (params (Sound :type Sound%20Wave%20Object%20Reference))
  (bind _playeraudio (Variables|Default|GetPlayerAudio))
  (Audio|Components|Audio|SetSound _playeraudio Sound)
  (Audio|Components|Audio|Play _playeraudio 0.0))

(event Custom|PlayAudioWithSubtitle
  (params (TrackName :type Name) (StartDelay :type Float%20%28single-precision%29))
  ;[1 1 1] Play an Audio Track with Subtitle
  (Default|PlaySubtitle (Variables|Default|GetSubtitleWidget) TrackName StartDelay))

(event Custom|HandleEnemyDied
  (params (WhoDied :type Enemy%20Character%20Object%20Reference))
  ;[1 1 1] Handle the enemy dieing event
  (AI|Components|Blackboard|SetValueasBool (AI|GetBlackboard WhoDied) (Variables|Default|GetEnemyAIActive) false)
  (AI|Navigation|StopMovement (Pawn|GetController WhoDied))
  (Utilities|Array|RemoveItem (Variables|Default|GetEnemies) WhoDied)
  (Default|DeathSequence WhoDied)
  (switch Utilities|FlowControl|Switch|SwitchonCurrentGameState (Variables|Default|GetCurrentGameState)
    (:NewEnumerator1
      _)
    (:NewEnumerator3
      _)
    (:NewEnumerator4
      _))
  (bind _cleared (CallFunction|IstheFloorCleared))
  (if _cleared
    (Variables|Default|SetCurrentGameState "NewEnumerator5")
    (CallFunction|HandleFloorCleared)
    (else
      (CallFunction|PlayEnemiesRemainingwithSub))))

(event Custom|ToggleInGameMenu
  (params (ForceOpen :type Boolean))
  (bind _returnvalue (Game|GetPlayerController 0))
  (bind _returnvalue_2 (Game|GetPlayerController 0))
  ;[1 1 1] Toggle the in game menu
  (if ForceOpen
    (bind _returnvalue_3 (UserInterface|CreateWidget "/Game/MyContent/Blueprints/UMG/InGameMenu.InGameMenu_C" :!label _label))
    (bind _output_get (Variables|Default|SetInGameMenuWidget _returnvalue_3))
    (bind _asin_game_menu (Utilities|Casting|CastToInGameMenu _output_get))
    (bind _returnvalue_4 (Game|GetCurrentLevelName true))
    (if (Utilities|Enum|Equal(Enum) _returnvalue_4 "Tutorial")
      (Widget|SetVisibility (Variables|/Game/MyContent/Blueprints/UMG/InGameMenu.InGameMenu_C|GetEnemiesLeftBox _asin_game_menu) "Hidden")
      (else
        (Rendering|Components|TextRender|SetText (Variables|/Game/MyContent/Blueprints/UMG/InGameMenu.InGameMenu_C|GetTBEnemiesLeft _asin_game_menu) (Utilities|Text|ToText(Integer) (Utilities|Array|Length (Variables|Default|GetEnemies))))))
    (UserInterface|Viewport|AddtoViewport (Variables|Default|GetInGameMenuWidget) 0)
    (Input|SetInputModeGameandUI _returnvalue_2 0 false true)
    (Variables|/Script/Engine.PlayerController|SetbShowMouseCursor _returnvalue_2 true)
    (if (not (Utilities|Enum|Equal(Enum) (Variables|Default|GetCurrentGameState) "NewEnumerator6"))
      (Variables|Default|SetCurrentGameState "NewEnumerator3"))
    (else
      (switch Utilities|FlowControl|Switch|SwitchonCurrentGameState (Variables|Default|GetCurrentGameState)
        (:NewEnumerator1
          _)
        (:NewEnumerator5
          _)
        (:NewEnumerator3
          _)
        (:NewEnumerator4
          _))
      (if (== (Variables|Default|GetInGameMenuWidget) 0)
        (goto _label)
        (else
          (Default|SaveSettings (.AsIn%20Game%20Menu (Utilities|Casting|CastToInGameMenu (Variables|Default|GetInGameMenuWidget))))
          (Widget|RemovefromParent (Variables|Default|GetInGameMenuWidget))
          (Variables|Default|SetInGameMenuWidget 0)
          (Input|SetInputModeGameOnly _returnvalue)
          (Variables|/Script/Engine.PlayerController|SetbShowMouseCursor _returnvalue false)
          (Variables|Default|SetCurrentGameState "NewEnumerator1"))))))

(event Custom|ChangeSoundVolume
  (params (LoadFromSave :type Boolean) (NewVolume :type Float%20%28single-precision%29))
  ;[1 1 1] Handle toggling the sound or volume changing
  (if LoadFromSave
    (bind _returnvalue (SaveGame|LoadGamefromSlot "SaveSlot"))
    (bind _asmy_save_game (Utilities|Casting|CastToMySaveGame _returnvalue)
      (:then
        (if (Variables|/Game/MyContent/Blueprints/Framework/MySaveGame.MySaveGame_C|GetSoundEnabled _asmy_save_game)
          (CallFunction|AdjustSoundVolume (Variables|/Game/MyContent/Blueprints/Framework/MySaveGame.MySaveGame_C|GetSoundVolume _asmy_save_game)) ; Failed so sound is on
          (else
            (CallFunction|AdjustSoundVolume 0.0) ; Failed so sound is on
          )))
      (:CastFailed
        (CallFunction|AdjustSoundVolume 1.0) ; Failed so sound is on
      ))
    (else
      (CallFunction|AdjustSoundVolume NewVolume))))

(event Custom|HandlePlayerDied
  (bind _enemies (Variables|Default|GetEnemies))
  ;[1 1 1] Handle Player Died
  (Input|DisableInput (Game|GetPlayerCharacter 0) (Game|GetPlayerController 0))
  (if (> (Utilities|Array|Length _enemies) 0)
    (for _array_element _enemies
      (AI|Components|Blackboard|SetValueasBool (AI|GetBlackboard _array_element) (Variables|Default|GetEnemyAIActive) false)
      (AI|Components|Blackboard|SetValueasBool (AI|GetBlackboard _array_element) (Variables|Default|GetEnemyAIAttackPlayer) false)
      (Variables|/Game/MyContent/Enemies/EnemyCharacter.EnemyCharacter_C|SetIsAlive _array_element false)
      (AI|Navigation|StopMovement (Pawn|GetController _array_element))))
  (bind _asrobot_character (Utilities|Casting|CastToRobotCharacter (Game|GetPlayerCharacter 0)))
  (Default|HandleDeathSequence _asrobot_character)
  (Variables|Default|SetCurrentGameState "NewEnumerator6")
  (CallFunction|ToggleinGameMenu true))

(event Custom|PlayEnemiesRemainingWithSub
  ;[1 1 1] Play an Audio Track with Subtitle showing enemies left in the level
  (Default|PlayEnemiesSubtitle (Variables|Default|GetSubtitleWidget) (Utilities|Array|Length (Variables|Default|GetEnemies))))

(event Custom|ChangeMusicVolume
  (params (LoadFromSave :type Boolean) (NewVolume :type Float%20%28single-precision%29))
  ;[1 1 1] Handle toggling the music or volume changing
  (if LoadFromSave
    (bind _returnvalue (SaveGame|LoadGamefromSlot "SaveSlot"))
    (bind _asmy_save_game (Utilities|Casting|CastToMySaveGame _returnvalue)
      (:then
        (if (Variables|/Game/MyContent/Blueprints/Framework/MySaveGame.MySaveGame_C|GetMusicEnabled _asmy_save_game)
          (CallFunction|AdjustMusicVolume (Variables|/Game/MyContent/Blueprints/Framework/MySaveGame.MySaveGame_C|GetMusicVolume _asmy_save_game))
          (else
            (CallFunction|AdjustMusicVolume 0.0))))
      (:CastFailed
        (CallFunction|AdjustMusicVolume 1.0)))
    (else
      (CallFunction|AdjustMusicVolume NewVolume))))

(event EventBeginPlay
  ;[1 1 1] Begin Play
  (CallFunction|CreateHUD)
  (CallFunction|InitializeLevel)
  (CallFunction|StarttheAI)
  (CallFunction|HandleSoundSetup))

(fn ConstructionScript)

(fn InitializeLevel
  (bind _outactors (Actor|GetAllActorsOfClass "/Game/MyContent/Enemies/EnemyCharacter.EnemyCharacter_C"))
  (Variables|Default|SetEnemies _outactors))

(fn CreateHUD
  (bind _returnvalue (UserInterface|CreateWidget "/Game/MyContent/Blueprints/UMG/TrapHUD.TrapHUD_C"))
  (bind _output_get (Variables|Default|SetTrapHUD _returnvalue))
  (UserInterface|Viewport|AddtoViewport _output_get 0)
  (Widget|SetVisibility (Variables|Default|GetTrapHUD) "Hidden")
  (bind _returnvalue_2 (UserInterface|CreateWidget "/Game/MyContent/Blueprints/UMG/SubtitlesHUD.SubtitlesHUD_C"))
  (bind _output_get_2 (Variables|Default|SetSubtitleWidget _returnvalue_2))
  (UserInterface|Viewport|AddtoViewport _output_get_2 0))

(fn EnemyDied
  (params (WhoDied :type Enemy%20Character%20Object%20Reference)))

(fn StarttheAI
  (for _array_element (Variables|Default|GetEnemies)
    (AI|Components|Blackboard|SetValueasBool (AI|GetBlackboard _array_element) (Variables|Default|GetEnemyAIActive) true)))

(fn IstheFloorCleared
  (return (<= (Utilities|Array|Length (Variables|Default|GetEnemies)) 0)))

(fn HandleFloorCleared
  (bind _outactors (Actor|GetAllActorsOfClass "/Game/MyContent/Blueprints/Manager/FloorManager.FloorManager_C"))
  (if (Utilities|IsValid (Utilities|Array|Get(acopy) _outactors))
    (Default|HandleFloorClearedEvent (Utilities|Array|Get(acopy) _outactors))))

(fn HandleSoundSetup
  (CallFunction|ChangeSoundVolume true 0.0)
  (CallFunction|ChangeMusicVolume true 0.0)
  (bind _asrobot_character (Utilities|Casting|CastToRobotCharacter (Game|GetPlayerCharacter 0)))
  (Audio|Components|Audio|SetSound (Variables|/Game/MyContent/Character/RobotCharacter.RobotCharacter_C|GetMusicComp _asrobot_character) (Variables|Default|GetMusicCue))
  (Audio|Components|Audio|Play (Variables|/Game/MyContent/Character/RobotCharacter.RobotCharacter_C|GetMusicComp _asrobot_character) 0.0)
  (Variables|Default|SetPlayerAudio (Variables|/Game/MyContent/Character/RobotCharacter.RobotCharacter_C|GetAudioComp _asrobot_character)))

(fn AdjustSoundVolume
  (params (NewVolume :type Float%20%28single-precision%29))
  (bind _asrobot_character (Utilities|Casting|CastToRobotCharacter (Game|GetPlayerCharacter 0)))
  (Audio|Components|Audio|SetVolumeMultiplier (Variables|/Game/MyContent/Character/RobotCharacter.RobotCharacter_C|GetAudioComp _asrobot_character) NewVolume :!class /Script/Engine.AudioComponent)
  (Audio|Components|Audio|SetVolumeMultiplier (Variables|/Game/MyContent/Character/RobotCharacter.RobotCharacter_C|GetSubComp _asrobot_character) NewVolume :!class /Script/Engine.AudioComponent)
  (return))

(fn AdjustMusicVolume
  (params (NewVolume :type Float%20%28single-precision%29))
  (bind _asrobot_character (Utilities|Casting|CastToRobotCharacter (Game|GetPlayerCharacter 0)))
  (Audio|Components|Audio|SetVolumeMultiplier (Variables|/Game/MyContent/Character/RobotCharacter.RobotCharacter_C|GetMusicComp _asrobot_character) NewVolume :!class /Script/Engine.AudioComponent)
  (return))