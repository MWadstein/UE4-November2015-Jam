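; Door actor that slides its Door component open or closed when its OpenDoor or CloseDoor event is called.
; BeginPlay caches the start and offset end locations and disables actor tick; separate timelines lerp between the two positions.
; A DoorMoving flag blocks new requests mid-motion.
; Sounds play through MyGameState, at the start when opening and from a timeline event track when closing.
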(event Custom|OpenDoor
  ;[1 1 1] Open Door
  (if (not (Variables|Default|GetDoorMoving))
    (Variables|Default|SetDoorMoving true)
    (bind _asmy_game_state (Utilities|Casting|CastToMyGameState (Game|GetGameState)))
    (Default|PlaySound _asmy_game_state "/Game/MyContent/Audio/FX/FX_DoorOpen.FX_DoorOpen")
    (bind _lerp_0___1 (Timeline|Timeline_0 PlayFromStart)
      (:Update
        (Transformation|SetWorldLocation (Variables|Default|GetDoor) (Math|Vector|Lerp(Vector) (Variables|Default|GetStartingLocation) (Variables|Default|GetEndingLocation) _lerp_0___1) false false))
      (:Finished
        (Variables|Default|SetDoorMoving false)))))

(event Custom|CloseDoor
  ;[1 1 1] Close Door
  (if (not (Variables|Default|GetDoorMoving))
    (Variables|Default|SetDoorMoving true)
    (bind _lerp_0___1 (Timeline|Timeline_1 PlayFromStart)
      (:Update
        (Transformation|SetWorldLocation (Variables|Default|GetDoor) (Math|Vector|Lerp(Vector) (Variables|Default|GetEndingLocation) (Variables|Default|GetStartingLocation) _lerp_0___1) false false))
      (:Finished
        (Variables|Default|SetDoorMoving false))
      (:PlaySound
        (bind _asmy_game_state (Utilities|Casting|CastToMyGameState (Game|GetGameState)))
        (Default|PlaySound _asmy_game_state "/Game/MyContent/Audio/FX/FX_DoorClose.FX_DoorClose")))))

(event EventBeginPlay
  ;[1 1 1] Begin Play, Cache our locations
  (bind _output_get (Variables|Default|SetStartingLocation (Transformation|GetWorldLocation (Variables|Default|GetDoor))))
  (Variables|Default|SetEndingLocation (+ _output_get (Variables|Default|GetOpeningOffset)))
  (Actor|Tick|SetActorTickEnabled false))

(fn ConstructionScript)