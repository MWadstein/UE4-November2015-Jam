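; Exit door Blueprint that slides open once and closes behind the player to finish a level.
; BeginPlay caches the mesh's start location and an offset end location, which two timelines lerp between to open and close it.
; OpenDoor plays its sound through MyGameState, guarded to run once.
; A trigger box detects actors implementing the Player interface, closes the door once, waits briefly, then tells the FloorManager to handle level completion.
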(event OnComponentBeginOverlap(Box)
  (params (OtherActor :type Actor%20Object%20Reference) (OtherComp :type Primitive%20Component%20Object%20Reference) (OtherBodyIndex :type Integer) (bFromSweep :type Boolean) (SweepResult :type Hit%20Result%20Structure%20%28by%20ref%29))
  ;[1 1 1] Begin Overlap when we have left the exit
  (if (Utilities|DoesObjectImplementInterface OtherActor "/Game/MyContent/Blueprints/Interfaces/Player.Player_C")
    (if (not (Variables|Default|GetDoorHasBeenClosed))
      (Variables|Default|SetDoorHasBeenClosed true)
      (CallFunction|CloseDoor)
      (Utilities|FlowControl|Delay 1.0)
      (bind _outactors (Actor|GetAllActorsOfClass "/Game/MyContent/Blueprints/Manager/FloorManager.FloorManager_C"))
      (Default|HandleFinishLevel (Utilities|Array|Get(acopy) _outactors)))))

(event Custom|OpenDoor
  ;[1 1 1] Open Door
  (if (not (Variables|Default|GetDoorHasBeenOpened))
    (Variables|Default|SetDoorHasBeenOpened true)
    (bind _asmy_game_state (Utilities|Casting|CastToMyGameState (Game|GetGameState)))
    (Default|PlaySound _asmy_game_state "/Game/MyContent/Audio/FX/FX_ExitDoorOpen.FX_ExitDoorOpen")
    (bind _lerp_0___1 (Timeline|Open%20The%20Door PlayFromStart)
      (:Update
        (Transformation|SetWorldLocation (Variables|Default|GetStaticMesh) (Math|Vector|Lerp(Vector) (Variables|Default|GetStartingLocation) (Variables|Default|GetEndingLocation) _lerp_0___1) false false)))))

(event Custom|CloseDoor
  ;[1 1 1] Close Door
  (bind _lerp_0___1 (Timeline|Timeline_0 PlayFromStart)
    (:Update
      (Transformation|SetWorldLocation (Variables|Default|GetStaticMesh) (Math|Vector|Lerp(Vector) (Variables|Default|GetEndingLocation) (Variables|Default|GetStartingLocation) _lerp_0___1) false false))))

(event EventBeginPlay
  ;[1 1 1] Begin Play, Cache our locations
  (bind _output_get (Variables|Default|SetStartingLocation (Transformation|GetWorldLocation (Variables|Default|GetStaticMesh))))
  (Variables|Default|SetEndingLocation (+ _output_get (Variables|Setup|GetOpeningOffset))))

(fn ConstructionScript)