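; DoorTrigger is a base interactable button that opens and closes a linked door.
; Toggle alternates the door via FlipFlop, ignoring input while it moves or the trigger is destroyed, then calls ExtraEvent, an empty hook for children.
; A dynamic material shows focus through glow strength and state through glow color.
; Focus also drives the TrapHUD widget from GameState, whose first line is recolored by active state.
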(event Custom|ExtraEvent
  ;[1 1 1] Stub for Children
)

(event EventBeginPlay
  ;[1 1 1] Begin Play
  (bind _returnvalue (Rendering|Material|CreateDynamicMaterialInstance "/Game/MyContent/Materials/TrapIndicatorMat.TrapIndicatorMat" :!class /Script/Engine.KismetMaterialLibrary))
  (bind _output_get (Variables|Default|SetDynamicMatInst _returnvalue))
  (Rendering|Material|SetMaterial (Variables|Default|GetButton) 0 _output_get)
  (Rendering|Material|SetVectorParameterValue (Variables|Default|GetDynamicMatInst) "GlowColor" (Variables|Default|GetInitialColor) :!class /Script/Engine.MaterialInstanceDynamic)
  (bind _asmy_game_state (Utilities|Casting|CastToMyGameState (Game|GetGameState)))
  (Variables|Default|SetUIWidget (Variables|/Game/MyContent/Blueprints/Framework/MyGameState.MyGameState_C|GetTrapHUD _asmy_game_state)))

(event EventIsFocused
  (params (True :type Boolean))
  ;[1 1 1] Event Focused
  (if (not (Variables|Default|GetIsDestroyed))
    (if True
      (Rendering|Material|SetScalarParameterValue (Variables|Default|GetDynamicMatInst) "GlowStrength" 4.0 :!class /Script/Engine.MaterialInstanceDynamic)
      (Widget|SetVisibility (Variables|Default|GetUIWidget) "Visible")
      (CallFunction|UpdateHUD1)
      (Rendering|Components|TextRender|SetText (Variables|/Game/MyContent/Blueprints/UMG/TrapHUD.TrapHUD_C|GetTBLine1 (Variables|Default|GetUIWidget)) (Variables|Default|GetHUDLine1))
      (Rendering|Components|TextRender|SetText (Variables|/Game/MyContent/Blueprints/UMG/TrapHUD.TrapHUD_C|GetTBLine2 (Variables|Default|GetUIWidget)) (Variables|Default|GetHUDLine2))
      (Rendering|Components|TextRender|SetText (Variables|/Game/MyContent/Blueprints/UMG/TrapHUD.TrapHUD_C|GetTBLine3 (Variables|Default|GetUIWidget)) (Variables|Default|GetHUDLine3))
      (else
        (Rendering|Material|SetScalarParameterValue (Variables|Default|GetDynamicMatInst) "GlowStrength" 0.5 :!class /Script/Engine.MaterialInstanceDynamic)
        (Widget|SetVisibility (Variables|Default|GetUIWidget) "Hidden")))))

(event EventToggle
  ;[1 1 1] Toggle Trap
  (if (not (Variables|/Game/MyContent/Blueprints/Environment/Door.Door_C|GetDoorMoving (Variables|Default|GetLinkedDoor)))
    (if (not (Variables|Default|GetIsDestroyed))
      (Utilities|FlowControl|FlipFlop
        (:A
          (Default|OpenDoor (Variables|Default|GetLinkedDoor))
          (Variables|Default|SetIsActive true)
          (Rendering|Material|SetVectorParameterValue (Variables|Default|GetDynamicMatInst) "GlowColor" (Variables|Default|GetOnColor) :!class /Script/Engine.MaterialInstanceDynamic)
          (CallFunction|UpdateHUD1))
        (:B
          (Default|CloseDoor (Variables|Default|GetLinkedDoor))
          (Variables|Default|SetIsActive false)
          (Rendering|Material|SetVectorParameterValue (Variables|Default|GetDynamicMatInst) "GlowColor" (Variables|Default|GetOffColor) :!class /Script/Engine.MaterialInstanceDynamic)
          (CallFunction|UpdateHUD1)))
      (CallFunction|ExtraEvent))))

(fn ConstructionScript)

(fn UpdateHUD1
  (Rendering|Components|TextRender|SetText (Variables|/Game/MyContent/Blueprints/UMG/TrapHUD.TrapHUD_C|GetTBLine1 (Variables|Default|GetUIWidget)) (Variables|Default|GetHUDLine1))
  (if (Variables|Default|GetIsActive)
    (Appearance|SetColorandOpacity (Variables|/Game/MyContent/Blueprints/UMG/TrapHUD.TrapHUD_C|GetTBLine1 (Variables|Default|GetUIWidget)) (LocalVariables|GetActiveColor) :!class /Script/UMG.TextBlock)
    (else
      (Appearance|SetColorandOpacity (Variables|/Game/MyContent/Blueprints/UMG/TrapHUD.TrapHUD_C|GetTBLine1 (Variables|Default|GetUIWidget)) (LocalVariables|GetInactiveColor) :!class /Script/UMG.TextBlock))))