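; Per-level floor manager that runs a floor's intro, clear and finish sequence with subtitled voice lines.
; On BeginPlay it saves the current floor and plays the intro once, tracked by a GameInstance flag, optionally locking player input meanwhile, then announces remaining enemies.
; Clearing the floor opens the assigned exit door.
; Finishing plays the ending line, waits out its subtitle delay, resets the intro flag and loads the next floor.
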(event Custom|HandleFloorClearedEvent
  ;[1 1 1] Handle clearing the floor
  (CallFunction|OpenExitDoor)
  (bind _asmy_game_state (Utilities|Casting|CastToMyGameState (Game|GetGameState)))
  (Default|PlayAudiowithSubtitle _asmy_game_state "Robot-EnemiesEliminated" 0.0))

(event Custom|DisablePlayerInputOnStart
  (bind _returnvalue (Game|GetPlayerCharacter 0))
  (bind _returnvalue_2 (Game|GetPlayerCharacter 0))
  ;[1 1 1] Disable player input on start, then wait for the intro to finish to turn it back on.
  (Input|DisableInput _returnvalue_2 (Game|GetPlayerController 0))
  (Default|ToggleNumberColor (.AsRobot%20Character (Utilities|Casting|CastToRobotCharacter _returnvalue_2)) false false)
  (bind _delay (CallFunction|GetSubDelay (Variables|Default|GetStartingAudioToPlay)))
  (Utilities|FlowControl|Delay _delay)
  (Input|EnableInput _returnvalue (Game|GetPlayerController 0))
  (Default|ToggleNumberColor (.AsRobot%20Character (Utilities|Casting|CastToRobotCharacter _returnvalue)) true true))

(event Custom|HandleFinishLevel
  ;[1 1 1] Handle Finishing the Level, loading the next
  (bind _asmy_game_state (Utilities|Casting|CastToMyGameState (Game|GetGameState)))
  (Default|PlayAudiowithSubtitle _asmy_game_state (Variables|Default|GetEndingAudioToPlay) 0.0)
  (bind _delay (CallFunction|GetSubDelay (Variables|Default|GetEndingAudioToPlay)))
  (Utilities|FlowControl|Delay _delay)
  (Variables|/Game/MyContent/Blueprints/Framework/MyGameInstance.MyGameInstance_C|SetPlayedLevelIntro (.AsMy%20Game%20Instance (Utilities|Casting|CastToMyGameInstance (Game|GetGameInstance))) false)
  (Game|OpenLevel(byName) (Variables|Setup|GetNextFloorName)))

(event EventBeginPlay
  ;[1 1 1] Begin Play
  (CallFunction|SaveCurrentFloor)
  (if (and (Variables|Setup|GetDisableInputOnStart) (not (Variables|/Game/MyContent/Blueprints/Framework/MyGameInstance.MyGameInstance_C|GetPlayedLevelIntro (.AsMy%20Game%20Instance (Utilities|Casting|CastToMyGameInstance (Game|GetGameInstance))))))
    (Utilities|Time|SetTimerbyFunctionName 0 "DisablePlayerInputOnStart" 0.1))
  (bind _asrobot_character (Utilities|Casting|CastToRobotCharacter (Game|GetPlayerCharacter 0)))
  (Default|BobRobot _asrobot_character)
  (if (Variables|/Game/MyContent/Blueprints/Framework/MyGameInstance.MyGameInstance_C|GetPlayedLevelIntro (.AsMy%20Game%20Instance (Utilities|Casting|CastToMyGameInstance (Game|GetGameInstance))))
    _
    (else
      (bind _asmy_game_state (Utilities|Casting|CastToMyGameState (Game|GetGameState)))
      (Default|PlayAudiowithSubtitle _asmy_game_state (Variables|Default|GetStartingAudioToPlay) 0.0)
      (bind _delay (CallFunction|GetSubDelay (Variables|Default|GetStartingAudioToPlay)))
      (Utilities|FlowControl|Delay _delay)
      (Variables|/Game/MyContent/Blueprints/Framework/MyGameInstance.MyGameInstance_C|SetPlayedLevelIntro (.AsMy%20Game%20Instance (Utilities|Casting|CastToMyGameInstance (Game|GetGameInstance))) true)))
  (bind _asmy_game_state_2 (Utilities|Casting|CastToMyGameState (Game|GetGameState)))
  (Default|PlayEnemiesRemainingwithSub _asmy_game_state_2))

(fn ConstructionScript)

(fn OpenExitDoor
  (if (Utilities|IsValid (Variables|Setup|GetExitDoor))
    (Default|OpenDoor (Variables|Setup|GetExitDoor))
    (else
      (Development|PrintString "You Forgot To assign an Exit Door"))))

(fn SaveCurrentFloor
  (bind _returnvalue (SaveGame|LoadGamefromSlot "SaveSlot"))
  (bind _asmy_save_game (Utilities|Casting|CastToMySaveGame _returnvalue)
    (:then
      (LocalVariables|SetSaveGameInst _asmy_save_game))
    (:CastFailed
      (bind _returnvalue_2 (SaveGame|CreateSaveGameObject "/Game/MyContent/Blueprints/Framework/MySaveGame.MySaveGame_C"))
      (bind _asmy_save_game_2 (Utilities|Casting|CastToMySaveGame _returnvalue_2))
      (LocalVariables|SetSaveGameInst _asmy_save_game_2)))
  (bind _returnvalue_3 (Game|GetCurrentLevelName true))
  (Variables|/Game/MyContent/Blueprints/Framework/MySaveGame.MySaveGame_C|SetCurrentFloor (LocalVariables|GetSaveGameInst) (Utilities|String|StringToName _returnvalue_3))
  (SaveGame|SaveGametoSlot (LocalVariables|GetSaveGameInst) "SaveSlot"))