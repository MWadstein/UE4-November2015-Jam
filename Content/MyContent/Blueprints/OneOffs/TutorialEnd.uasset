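; Tutorial exit trigger that ends the tutorial and moves the game to the next level.
; When an actor implementing the Player interface overlaps its box, it disables player input and has MyGameState play the robot's tutorial-end audio with a subtitle.
; It waits for that line's subtitle delay, then opens the level named by NextLevel.
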(event OnComponentBeginOverlap(Box)
  (params (OtherActor :type Actor%20Object%20Reference) (OtherComp :type Primitive%20Component%20Object%20Reference) (OtherBodyIndex :type Integer) (bFromSweep :type Boolean) (SweepResult :type Hit%20Result%20Structure%20%28by%20ref%29))
  ;[1 1 1] Disable Input and start the subtile for the end of the tutorial
  (if (Utilities|DoesObjectImplementInterface OtherActor "/Game/MyContent/Blueprints/Interfaces/Player.Player_C")
    (Input|DisableInput (Game|GetPlayerCharacter 0) (Game|GetPlayerController 0))
    (Default|PlayAudiowithSubtitle (.AsMy%20Game%20State (Utilities|Casting|CastToMyGameState (Game|GetGameState))) "Robot-TutorialEnd" 0.0) ; Tutorial End
    (bind _delay (CallFunction|GetSubDelay "Robot-TutorialEnd"))
    (Utilities|FlowControl|Delay _delay)
    (Game|OpenLevel(byName) (Variables|Setup|GetNextLevel))))

(fn ConstructionScript)