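; Runs the robot tutorial intro on BeginPlay, starting with player input locked, music and exhaust off, and the robot mesh lowered.
; A spawned camera blends to the player while a chain of voiceover tracks plays through MyGameState, each paced by its subtitle delay.
; After the first line, exhaust activates and a timeline lifts the mesh into bobbing.
; Later lines progressively restore look input, then movement and the flashing number color.
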(event Custom|PlayVoiceoverSequence
  ;[1 1 1] Insanely long event for the startup subtitles and letting regain control over time
  (Default|PlayAudiowithSubtitle (Variables|Default|GetMyGS) "Robot-Tutorial1" 0.0) ; Part 1
  (bind _delay (CallFunction|GetSubDelay "Robot-Tutorial1"))
  (Utilities|FlowControl|Delay _delay)
  (bind _asrobot_character (Utilities|Casting|CastToRobotCharacter (Game|GetPlayerCharacter 0)))
  (Components|Activation|SetActive (Variables|/Game/MyContent/Character/RobotCharacter.RobotCharacter_C|GetExhaust _asrobot_character) true true)
  (bind _output_get (Variables|Default|SetPlayerMesh (Variables|/Script/Engine.Character|GetMesh _asrobot_character)))
  (Variables|Default|SetMeshStartingLocation (Variables|/Script/Engine.SceneComponent|GetRelativeLocation _output_get))
  (Variables|Default|SetMeshEndingLocation (+ (Variables|/Script/Engine.SceneComponent|GetRelativeLocation _output_get) "0, 0,45.000000"))
  (bind _lerp_0_1 (Timeline|ActivateExhaustTimeline PlayFromStart)
    (:Update
      (Transformation|SetRelativeLocation (Variables|Default|GetPlayerMesh) (Math|Vector|Lerp(Vector) (Variables|Default|GetMeshStartingLocation) (Variables|Default|GetMeshEndingLocation) _lerp_0_1) false false))
    (:Finished
      (bind _asrobot_character_2 (Utilities|Casting|CastToRobotCharacter (Game|GetPlayerCharacter 0)))
      (Default|BobRobot _asrobot_character_2)
      (Default|PlayAudiowithSubtitle (Variables|Default|GetMyGS) "Robot-Tutorial2" 0.0) ; Part 2
      (bind _delay_2 (CallFunction|GetSubDelay "Robot-Tutorial2"))
      (Utilities|FlowControl|Delay _delay_2)
      (Input|ResetIgnoreLookInput (Game|GetPlayerController 0))
      (Default|PlayAudiowithSubtitle (Variables|Default|GetMyGS) "Robot-Tutorial3" 1.0) ; Part 3
      (bind _delay_3 (CallFunction|GetSubDelay "Robot-Tutorial3"))
      (Utilities|FlowControl|Delay (+ _delay_3 1.0))
      (Default|PlayAudiowithSubtitle (Variables|Default|GetMyGS) "Robot-Tutorial4" 1.0) ; Part 4
      (bind _delay_4 (CallFunction|GetSubDelay "Robot-Tutorial4"))
      (Utilities|FlowControl|Delay (+ _delay_4 1.0))
      (Default|PlayAudiowithSubtitle (Variables|Default|GetMyGS) "Robot-Tutorial5" 1.0) ; Part 5
      (bind _delay_5 (CallFunction|GetSubDelay "Robot-Tutorial5"))
      (Utilities|FlowControl|Delay (+ _delay_5 1.0))
      (Input|ResetIgnoreMoveInput (Game|GetPlayerController 0))
      (Default|ToggleNumberColor (.AsRobot%20Character (Utilities|Casting|CastToRobotCharacter (Game|GetPlayerCharacter 0))) true true)
      (Default|PlayAudiowithSubtitle (Variables|Default|GetMyGS) "Robot-Tutorial6" 1.0) ; Part 6
      (bind _delay_6 (CallFunction|GetSubDelay "Robot-Tutorial6"))
      (Utilities|FlowControl|Delay (+ _delay_6 1.0))
      (Default|PlayAudiowithSubtitle (Variables|Default|GetMyGS) "Robot-Tutorial7" 1.0) ; Part 7
      (bind _delay_7 (CallFunction|GetSubDelay "Robot-Tutorial7"))
      (Utilities|FlowControl|Delay _delay_7))))

(event EventBeginPlay
  (bind _returnvalue (Game|GetPlayerController 0))
  (bind _returnvalue_2 (Game|GetPlayerController 0))
  ;[1 1 1] Start our tutorial sequence
  (bind _asrobot_character (Utilities|Casting|CastToRobotCharacter (Game|GetPlayerCharacter 0)))
  (Default|ToggleNumberColor _asrobot_character false false)
  (Audio|Components|Audio|Stop (Variables|/Game/MyContent/Character/RobotCharacter.RobotCharacter_C|GetMusicComp _asrobot_character))
  (Components|Activation|SetActive (Variables|/Game/MyContent/Character/RobotCharacter.RobotCharacter_C|GetExhaust _asrobot_character) false true)
  (Input|SetIgnoreMoveInput _returnvalue_2 true)
  (Input|SetIgnoreLookInput _returnvalue_2 true)
  (bind _asmy_game_state (Utilities|Casting|CastToMyGameState (Game|GetGameState)))
  (Variables|Default|SetMyGS _asmy_game_state)
  (bind _asrobot_character_2 (Utilities|Casting|CastToRobotCharacter (Game|GetPlayerCharacter 0)))
  (Transformation|AddWorldOffset (Variables|/Script/Engine.Character|GetMesh _asrobot_character_2) "0, 0,-45.000000" false false)
  (bind _returnvalue_3 (Game|SpawnActorfromClass "/Script/Engine.CameraActor" (Math|Transform|MakeTransform "205.000000,1165.000000,600.000000" "-50.000000,-70.000000,0.000000" "1,1,1") "Undefined" 0 0)) ; Spawn our starting camera for blend
  (Variables|/Script/Engine.CameraComponent|SetbConstrainAspectRatio (Variables|/Script/Engine.CameraActor|GetCameraComponent _returnvalue_3) false)
  (Game|Player|SetViewTargetwithBlend _returnvalue _returnvalue_3 0.0 "VTBlend_Linear" 0.0 false) ; Change to new camera
  (Game|Player|SetViewTargetwithBlend _returnvalue (Game|GetPlayerCharacter 0) 5.0 "VTBlend_Cubic" 6.0 false) ; Blend to player
  (Utilities|FlowControl|Delay 1.3)
  (CallFunction|PlayVoiceoverSequence))

(fn ConstructionScript)